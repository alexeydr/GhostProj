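; BP_InteractActor is an interactable item actor that handles interaction prompts and menus.
; OnInteract shows a "Press E" prompt with the item name, clearing its reference after a one-second delay without removing the widget here.
; CreateInteractWidget opens a single item menu linked to this actor, shows the cursor and disables player movement.
; PlayEffect displays a usage UI and sets movement to Walking immediately after disabling it.
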(event `self.PlayEffect`
  (bind _charactermovement (`Character.CharacterMovement` (`GameplayStatics.GetPlayerCharacter` 0)))
  (bind _returnvalue (`|CreateWidget` "/Game/Widget/UsageUI.UsageUI_C"))
  (`UserWidget.AddToViewport` _returnvalue 0)
  (`CharacterMovementComponent.DisableMovement` _charactermovement)
  (`CharacterMovementComponent.SetMovementMode` _charactermovement "MOVE_Walking" 0))

(event `self.CreateInteractWidget`
  (if (not (`KismetSystemLibrary.IsValid` (`self.InteractWidget`)))
    (bind _returnvalue (`|CreateWidget` "/Game/Widget/InteractWithItemMenu.InteractWithItemMenu_C"))
    (set `self.InteractWidget` _returnvalue)
    (set `/Game/Widget/InteractWithItemMenu.Item` self _returnvalue)
    (`UserWidget.AddToViewport` _returnvalue 0)
    (set `PlayerController.bShowMouseCursor` true (`GameplayStatics.GetPlayerController` 0))
    (`CharacterMovementComponent.DisableMovement` (`Character.CharacterMovement` (`GameplayStatics.GetPlayerCharacter` 0)))))

(event `self.OnInteract`
  (params (Name :type String))
  (`/Engine/EditorBlueprintResources/StandardMacros.IsValid` (`self.InfoInteract`)
    (:`Is Not Valid`
      (bind _returnvalue (`|CreateWidget` "/Game/Widget/Info/InteractWidget.InteractWidget_C"))
      (`UserWidget.AddToViewport` _returnvalue 0)
      (bind _output_get (set `self.InfoInteract` _returnvalue))
      (`TextBlock.SetText` (`/Game/Widget/Info/InteractWidget.TextBlock_148` _output_get) (`KismetTextLibrary.Conv_StringToText` (`KismetStringLibrary.Concat_StrStr` "Press E to interact with " Name)))
      (`KismetSystemLibrary.Delay` 1.0)
      (set `self.InfoInteract` null))))

(fn `UserConstructionScript`)