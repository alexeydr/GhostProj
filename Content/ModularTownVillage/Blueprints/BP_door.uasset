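; Village door actor with selectable decoration and open or closed state, opened and closed through custom events.
; The construction script sets the door's starting yaw from Open and picks a plain or decorated dynamic material.
; For decorated doors, it tints the decoration with DecoColor and swaps mask and normal textures per DecoType.
; Open_the_door plays a timeline that drives the mesh's relative yaw, and CLose_the_door reverses it.
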(event `self.ReceiveBeginPlay`)

(event `Open_the_door`
  ;[1 1 1] Use these events when you want to open or to close the door
  (bind (_direction _z_rotation) (`Timeline|Timeline_open_door` :!label _label)
    (:`Update`
      (`SceneComponent.K2_SetRelativeRotation` (`self.SM_door`) (`KismetMathLibrary.MakeRotator` 0.0 0.0 _z_rotation) false false))))

(event `CLose_the_door`
  ;[1 1 1] Use these events when you want to open or to close the door
  (goto _label :!via `Reverse`))

(fn `UserConstructionScript`
  (bind _door_dynamic_mat (`self.door_dynamic_mat`))
  (bind _door_dynamic_mat_2 (`self.door_dynamic_mat`))
  (bind _door_dynamic_mat_3 (`self.door_dynamic_mat`))
  (bind _door_dynamic_mat_4 (`self.door_dynamic_mat`))
  (bind _sm_door (`self.SM_door`))
  (bind _door_dynamic_mat_5 (`self.door_dynamic_mat`))
  (bind _door_dynamic_mat_6 (`self.door_dynamic_mat`))
  (bind _door_dynamic_mat_7 (`self.door_dynamic_mat`))
  (bind _door_dynamic_mat_8 (`self.door_dynamic_mat`))
  (bind _door_dynamic_mat_9 (`self.door_dynamic_mat`))
  (if (`|EnumEquality` (`self.deco type`) "NewEnumerator0")
    (`PrimitiveComponent.CreateDynamicMaterialInstance` (`self.SM_door`) 0 "/Game/ModularTownVillage/Materials/MI_door.MI_door")
    (else
      (bind _returnvalue (`PrimitiveComponent.CreateDynamicMaterialInstance` (`self.SM_door`) 0 "/Game/ModularTownVillage/Materials/MI_door_deco.MI_door_deco"))
      (set `self.door_dynamic_mat` _returnvalue)
      (`MaterialInstanceDynamic.SetVectorParameterValue` (`self.door_dynamic_mat`) "deco tint" (`self.deco color`))))
  (if (`self.open?`)
    (`SceneComponent.K2_SetRelativeRotation` _sm_door (`KismetMathLibrary.MakeRotator` 0.0 0.0 -120.0) false false)
    (else
      (`SceneComponent.K2_SetRelativeRotation` _sm_door (`KismetMathLibrary.MakeRotator` 0.0) false false)))
  (switch `/Game/ModularTownVillage/Blueprints/E_deco_door` (`self.deco type`)
    (:`NewEnumerator1`
      (`MaterialInstanceDynamic.SetTextureParameterValue` _door_dynamic_mat_2 "Deco_mask" "/Game/ModularTownVillage/Textures/T_deco_flower_Mask.T_deco_flower_Mask")
      (`MaterialInstanceDynamic.SetTextureParameterValue` _door_dynamic_mat_2 "Deco Normal" "/Game/ModularTownVillage/Textures/T_deco_N_01.T_deco_N_01"))
    (:`NewEnumerator2`
      (`MaterialInstanceDynamic.SetTextureParameterValue` _door_dynamic_mat_3 "Deco_mask" "/Game/ModularTownVillage/Textures/T_deco_cross_Mask.T_deco_cross_Mask")
      (`MaterialInstanceDynamic.SetTextureParameterValue` _door_dynamic_mat_3 "Deco Normal" "/Game/ModularTownVillage/Textures/T_deco_N_02.T_deco_N_02"))
    (:`NewEnumerator3`
      (`MaterialInstanceDynamic.SetTextureParameterValue` _door_dynamic_mat_4 "Deco_mask" "/Game/ModularTownVillage/Textures/T_deco_celtic_cross_Mask.T_deco_celtic_cross_Mask")
      (`MaterialInstanceDynamic.SetTextureParameterValue` _door_dynamic_mat_4 "Deco Normal" "/Game/ModularTownVillage/Textures/T_deco_N_03.T_deco_N_03"))
    (:`NewEnumerator9`
      (`MaterialInstanceDynamic.SetTextureParameterValue` _door_dynamic_mat_5 "Deco_mask" "/Game/ModularTownVillage/Textures/T_deco_celtic_cross_butterfly_Mask.T_deco_celtic_cross_butterfly_Mask")
      (`MaterialInstanceDynamic.SetTextureParameterValue` _door_dynamic_mat_5 "Deco Normal" "/Game/ModularTownVillage/Textures/T_deco_N_04.T_deco_N_04"))
    (:`NewEnumerator4`
      (`MaterialInstanceDynamic.SetTextureParameterValue` _door_dynamic_mat_6 "Deco_mask" "/Game/ModularTownVillage/Textures/T_deco_fleur_de_lis_Mask.T_deco_fleur_de_lis_Mask")
      (`MaterialInstanceDynamic.SetTextureParameterValue` _door_dynamic_mat_6 "Deco Normal" "/Game/ModularTownVillage/Textures/T_deco_N_05.T_deco_N_05"))
    (:`NewEnumerator5`
      (`MaterialInstanceDynamic.SetTextureParameterValue` _door_dynamic_mat_7 "Deco_mask" "/Game/ModularTownVillage/Textures/T_deco_fish_Mask.T_deco_fish_Mask")
      (`MaterialInstanceDynamic.SetTextureParameterValue` _door_dynamic_mat_7 "Deco Normal" "/Game/ModularTownVillage/Textures/T_deco_N_06.T_deco_N_06"))
    (:`NewEnumerator6`
      (`MaterialInstanceDynamic.SetTextureParameterValue` _door_dynamic_mat_8 "Deco_mask" "/Game/ModularTownVillage/Textures/T_deco_lion_Mask.T_deco_lion_Mask")
      (`MaterialInstanceDynamic.SetTextureParameterValue` _door_dynamic_mat_8 "Deco Normal" "/Game/ModularTownVillage/Textures/T_deco_N_07.T_deco_N_07"))
    (:`NewEnumerator7`
      (`MaterialInstanceDynamic.SetTextureParameterValue` _door_dynamic_mat_9 "Deco_mask" "/Game/ModularTownVillage/Textures/T_deco_fire_Mask.T_deco_fire_Mask")
      (`MaterialInstanceDynamic.SetTextureParameterValue` _door_dynamic_mat_9 "Deco Normal" "/Game/ModularTownVillage/Textures/T_deco_N_08.T_deco_N_08"))
    (:`NewEnumerator8`
      (`MaterialInstanceDynamic.SetTextureParameterValue` _door_dynamic_mat "Deco_mask" "/Game/ModularTownVillage/Textures/T_deco_forge_Mask.T_deco_forge_Mask")
      (`MaterialInstanceDynamic.SetTextureParameterValue` _door_dynamic_mat "Deco Normal" "/Game/ModularTownVillage/Textures/T_deco_N_09.T_deco_N_09"))))