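; BP_SmallInteractActor is an item actor that shows an interaction prompt when its OnInteract event fires with a name.
; If InfoInteract holds no valid widget, it creates an InteractWidget, adds it to the viewport and sets its text to "Press E to interact with" plus the name.
; It clears the InfoInteract reference after a one-second delay, without removing the widget from the viewport.
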(event `self.OnInteract`
  (params (Name :type String))
  (`/Engine/EditorBlueprintResources/StandardMacros.IsValid` (`self.InfoInteract`)
    (:`Is Not Valid`
      (bind _returnvalue (`|CreateWidget` "/Game/Widget/Info/InteractWidget.InteractWidget_C"))
      (`UserWidget.AddToViewport` _returnvalue 0)
      (set `self.InfoInteract` _returnvalue)
      (`TextBlock.SetText` (`/Game/Widget/Info/InteractWidget.TextBlock_148` _returnvalue) (`KismetTextLibrary.Conv_StringToText` (`KismetStringLibrary.Concat_StrStr` "Press E to interact with " Name)))
      (`KismetSystemLibrary.Delay` 1.0)
      (set `self.InfoInteract` null))))

(fn `UserConstructionScript`)