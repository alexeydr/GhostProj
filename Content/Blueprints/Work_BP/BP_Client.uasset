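; BP_Client shows an on-screen "Press E to interact with" prompt for a named target when OnInteract fires.
; If no prompt reference is held, it creates an InteractWidget, adds it to the viewport and appends the passed name to its text.
; After a one-second delay it clears the reference to allow another prompt, without removing the widget from the viewport itself.
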(event `self.OnInteract`
  (params (Name :type String))
  (`/Engine/EditorBlueprintResources/StandardMacros.IsValid` (`self.InteractWidget`)
    (:`Is Not Valid`
      (bind _returnvalue (`|CreateWidget` "/Game/Widget/Info/InteractWidget.InteractWidget_C"))
      (`UserWidget.AddToViewport` _returnvalue 0)
      (bind _output_get (set `self.InteractWidget` _returnvalue))
      (`TextBlock.SetText` (`/Game/Widget/Info/InteractWidget.TextBlock_148` _output_get) (`KismetTextLibrary.Conv_StringToText` (`KismetStringLibrary.Concat_StrStr` "Press E to interact with " Name)))
      (`KismetSystemLibrary.Delay` 1.0)
      (set `self.InteractWidget` null))))

(fn `UserConstructionScript`)