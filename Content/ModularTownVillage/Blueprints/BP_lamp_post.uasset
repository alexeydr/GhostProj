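; Lamp post prop for the modular town village, pairing a static mesh with a point light.
; The construction script creates a dynamic material instance on the mesh, applies one color to its emissive tint and the light, and sets both on or off from the LightOff flag.
; Turn on and turn off events switch the material's emissive intensity and the light's intensity together, using the exposed intensity variables or zero.
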(event `self.ReceiveBeginPlay`)

(event `Turn_off_the_light`
  ;[1 1 1] Use these events to turn on/off the light. Intensity variables shouldn't be zero
  (`MaterialInstanceDynamic.SetScalarParameterValue` (`self.lamp_pose_dyn_mat_instance`) "emissive intensity" 0.0)
  (`LightComponent.SetIntensity` (`self.PointLight`) 0.0))

(event `Turn_on_the_light`
  ;[1 1 1] Use these events to turn on/off the light. Intensity variables shouldn't be zero
  (`MaterialInstanceDynamic.SetScalarParameterValue` (`self.lamp_pose_dyn_mat_instance`) "emissive intensity" (`self.emisive intensity`))
  (`LightComponent.SetIntensity` (`self.PointLight`) (`self.lamp_intensity`)))

(fn `UserConstructionScript`
  (bind _returnvalue (`PrimitiveComponent.CreateDynamicMaterialInstance` (`self.SM_lamp_post`) 0 "/Game/ModularTownVillage/Materials/MI_lamp_post.MI_lamp_post"))
  (set `self.lamp_pose_dyn_mat_instance` _returnvalue)
  (`MaterialInstanceDynamic.SetVectorParameterValue` (`self.lamp_pose_dyn_mat_instance`) "emisive tint" (`self.light_color`))
  (`LightComponent.SetLightColor` (`self.PointLight`) (`self.light_color`) true)
  (if (`self.light_off?`)
    (`MaterialInstanceDynamic.SetScalarParameterValue` (`self.lamp_pose_dyn_mat_instance`) "emissive intensity" 0.0)
    (`LightComponent.SetIntensity` (`self.PointLight`) 0.0)
    (else
      (`MaterialInstanceDynamic.SetScalarParameterValue` (`self.lamp_pose_dyn_mat_instance`) "emissive intensity" (`self.emisive intensity`))
      (`LightComponent.SetIntensity` (`self.PointLight`) (`self.lamp_intensity`)))))